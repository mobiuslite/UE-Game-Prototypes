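; Spleef game modifier that raises attack speed for the players it is applied to, using the Gameplay Ability System.
; On apply, it runs the parent logic, then applies the attack speed increase Gameplay Effect to each player with a valid Ability System Component.
; On destroy, it runs the parent logic, then removes all stacks of that effect from each player passed in.
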(event `self.ApplyModifier`
  (params (Players :type "Array of Actor Object Reference (by ref)"))
  (`parent.ApplyModifier` Players)
  (for _array_element Players
    (bind _returnvalue (`AbilitySystemBlueprintLibrary.GetAbilitySystemComponent` _array_element))
    (`/Engine/EditorBlueprintResources/StandardMacros.IsValid` _returnvalue
      (:`Is Valid`
        (`AbilitySystemComponent.BP_ApplyGameplayEffectToSelf` :`self` _returnvalue :`GameplayEffectClass` "/Game/Boxel/Core/SpleefGame/Modifiers/GameplayEffects/GE_AttackSpeed_Increase.GE_AttackSpeed_Increase_C")))))

(event `self.DestroyModifier`
  (params (Players :type "Array of Actor Object Reference (by ref)"))
  (`parent.DestroyModifier` Players)
  (for _array_element Players
    (bind _returnvalue (`AbilitySystemBlueprintLibrary.GetAbilitySystemComponent` _array_element))
    (`/Engine/EditorBlueprintResources/StandardMacros.IsValid` _returnvalue
      (:`Is Valid`
        (`AbilitySystemComponent.RemoveActiveGameplayEffectBySourceEffect` _returnvalue "/Game/Boxel/Core/SpleefGame/Modifiers/GameplayEffects/GE_AttackSpeed_Increase.GE_AttackSpeed_Increase_C" null -1)))))