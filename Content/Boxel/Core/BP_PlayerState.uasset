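; Player state that implements in-game voice chat through Steam voice functions.
; Speaking changes on the local controller start or stop Steam recording, and Tick polls captured voice data along with the Steam ID.
; Data passes through ReceivedVoice and SendVoice to ApplyVoiceData, which skips the player's own ID and decompresses into a procedural sound wave.
; The Audio component receives that wave and starts playback when it has no sound assigned.
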(event `self.ReceiveBeginPlay`
  (bind _returnvalue (`|GenericCreateObject` "/Script/Engine.SoundWaveProcedural"))
  (set `self.TalkingSoundWave` _returnvalue))

(event `self.OnSetSpeaking`
  (params (bSpeaking :type Boolean))
  (bind _returnvalue (`self.GetPlayerController`))
  (`parent.OnSetSpeaking` bSpeaking)
  (`/Engine/EditorBlueprintResources/StandardMacros.IsValid` _returnvalue
    (:`Is Valid`
      (if (`Controller.IsLocalController` _returnvalue)
        (`ToolkitSteamworksBPLibrary.SteamSetInGameVoiceSpeaking` bSpeaking)
        (if bSpeaking
          (`ToolkitSteamworksBPLibrary.SteamStartVoiceRecording`)
          (else
            (`ToolkitSteamworksBPLibrary.SteamStopVoiceRecording`)))))))

(event `self.ReceiveTick`
  (params (DeltaSeconds :type "Float (single-precision)"))
  (bind _returnvalue (`self.GetPlayerController`))
  (`/Engine/EditorBlueprintResources/StandardMacros.IsValid` _returnvalue
    (:`Is Valid`
      (if (`Controller.IsLocalPlayerController` _returnvalue)
        (bind _returnvalue_2 (`ToolkitSteamworksBPLibrary.SteamGetVoice`))
        (switch `UEVoiceResult` (break `VoiceResult` _returnvalue_2)
          (:`EPC_OK`
            (bind _returnvalue_3 (`ToolkitSteamworksBPLibrary.SteamGetMySteamId`))
            (`self.ReceivedVoice` _returnvalue_3 (`.VoiceData` (break `VoiceResult` _returnvalue_2)))))))))

(event `ReceivedVoice`
  (params (SteamID :type Integer64) (Data :type "Array of Byte"))
  (`self.SendVoice` SteamID Data))

(event `SendVoice`
  (params (SteamID :type Integer64) (Data :type "Array of Byte"))
  (`self.ApplyVoiceData` SteamID Data))

(fn `ApplyVoiceData`
  (params (SteamID :type Integer64) (Data :type "Array of Byte"))
  (bind _returnvalue (`ToolkitSteamworksBPLibrary.SteamGetMySteamId`))
  (if (!= _returnvalue SteamID)
    (bind _returnvalue_2 (`ToolkitSteamworksBPLibrary.SteamGetVoiceOptimalSampleRate`))
    (bind _returnvalue_3 (`ToolkitSteamworksBPLibrary.SteamDecompressVoice` Data _returnvalue_2 (`self.TalkingSoundWave`)))
    (if (break `DecompressVoiceResult` _returnvalue_3)
      (`/Engine/EditorBlueprintResources/StandardMacros.IsValid` (`AudioComponent.Sound` (`self.Audio`))
        (:`Is Not Valid`
          (`AudioComponent.SetSound` (`self.Audio`) (`self.TalkingSoundWave`))
          (if (not (`AudioComponent.IsPlaying` (`self.Audio`)))
            (`AudioComponent.Play` (`self.Audio`) 0.0)
            (`KismetSystemLibrary.PrintString` "Playing!")))))))

(fn `UserConstructionScript`)