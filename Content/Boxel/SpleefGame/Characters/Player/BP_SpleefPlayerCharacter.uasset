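; Player character for the Spleef game that handles local first-person presentation and landing feedback.
; On restart, the local player gets a hidden mesh and game-only input.
; Local landings after enough airtime trigger a camera shake and kick a float spring, both scaled by clamped airtime.
; Tick advances that damped spring into ExtraViewRotation, so the view bounces on impact and settles.
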(event `self.ReceiveRestarted`
  (`SceneComponent.SetVisibility` (`self.Mesh`) (not (`self.IsLocallyControlled`)) false)
  (if (`self.IsLocallyControlled`)
    (`WidgetBlueprintLibrary.SetInputMode_GameOnly` (cast `PlayerController` (`self.GetController`) :!pure true))))

(event `self.OnLandedEX`
  (params (TimeInAir :type "Float (single-precision)") (Hit :type "HitResult Structure (by ref)"))
  (bind _returnvalue (`KismetMathLibrary.FClamp` TimeInAir 0.0 (`self.MaxLandScreenShakeScale`)))
  (if (`self.IsLocallyControlled`)
    (if (> TimeInAir (`self.LandShakeThreshold`))
      (`PlayerCameraManager.StartCameraShake` :`self` (`GameplayStatics.GetPlayerCameraManager` 0) :`ShakeClass` "/Game/Boxel/Core/SpleefGame/Camera/CS_Landed.CS_Landed_C" :`Scale` _returnvalue)
      (`KismetMathLibrary.SetFloatSpringStateVelocity` (`self.Spring State`) (* _returnvalue (`self.LandCameraForce`))))))

(event `self.ReceiveTick`
  (params (DeltaSeconds :type "Float (single-precision)"))
  (bind _returnvalue (`KismetMathLibrary.FloatSpringInterp` (`self.DownTest`) 0.0 (`self.Spring State`) 100.0 0.65 DeltaSeconds 1.0 1.0 false -180.0 180.0 true))
  (bind _output_get (set `self.DownTest` _returnvalue))
  (set `self.ExtraViewRotation` (`KismetMathLibrary.MakeRotator` 0.0 _output_get)))

(fn `UserConstructionScript`)